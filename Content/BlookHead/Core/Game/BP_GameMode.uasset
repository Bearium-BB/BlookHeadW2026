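; BP_GameMode is the game mode that sets up the HUD and provides a distance-based score for the player.
; BeginPlay creates the WPB_HUD widget, switches to game-only input with a hidden cursor, and caches the BP_Player pawn.
; GetScroe returns the player's X location divided by 100 and rounded.
; Level completion, next-level loading, restart and game-completed functions are empty stubs.
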(event EventBeginPlay
  (bind _returnvalue (Game|GetPlayerController 0))
  (Utilities|FlowControl|Sequence
    (:then_0
      (bind _returnvalue_2 (UserInterface|CreateWidget "/Game/BlookHead/Core/UI/WPB_HUD.WPB_HUD_C"))
      (bind _output_get (Variables|Default|SetHUD _returnvalue_2))
      (UserInterface|Viewport|AddtoViewport _output_get 0))
    (:then_1
      (Input|SetInputModeGameOnly _returnvalue false)
      (Variables|/Script/Engine.PlayerController|SetbShowMouseCursor _returnvalue false))
    (:then_2
      (bind _asbp_player (Utilities|Casting|CastToBP_Player (Game|Player|GetPlayerPawn 0)))
      (Variables|Default|SetPlayer _asbp_player))))

(event EventTick
  (params (DeltaSeconds :type Float%20%28single-precision%29)))

(fn ConstructionScript)

(fn GetScroe
  (return (Math|Float|Round (/ (.x (Transformation|GetActorLocation (Variables|Default|GetPlayer))) 1e+02))))

(fn LevelComplete)

(fn LoadNextLevel)

(fn RestarGame)

(fn GameCompleted)