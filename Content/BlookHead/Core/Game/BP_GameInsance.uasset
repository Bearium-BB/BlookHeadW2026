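; Game instance Blueprint for BlookHead that holds the current level number and score and provides level-progression helpers.
; It can reset progress, advance the level, check for the final level, and build level names by appending the number to "Level0".
; Two input helpers switch between game-only input and UI-only input, toggling the mouse cursor and pause state together.
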(fn ResetInstance
  (Variables|Default|SetCurrentLevel 1)
  (Variables|Default|SetScroe 0.0)
  (return))

(fn NextLevel
  (Math|Integer|IncrementInt (Variables|Default|GetCurrentLevel)
    (:%20%20
      (return))))

(fn GetLevelName
  (return (Utilities|String|StringToName (Utilities|String|BuildString(Integer) "" "Level0" (Variables|Default|GetCurrentLevel)))))

(fn IsPlayeronFinalLevel
  (return (== (Variables|Default|GetCurrentLevel) (Variables|Default|GetMaxLevel))))

(fn InputGameMode
  (bind _returnvalue (Game|GetPlayerController 0))
  (Variables|/Script/Engine.PlayerController|SetbShowMouseCursor _returnvalue false)
  (Input|SetInputModeGameOnly _returnvalue false)
  (Game|SetGamePaused false)
  (return))

(fn InputModeUI
  (bind _returnvalue (Game|GetPlayerController 0))
  (Variables|/Script/Engine.PlayerController|SetbShowMouseCursor _returnvalue true)
  (Input|SetInputModeUIOnly _returnvalue 0 "DoNotLock" false)
  (Game|SetGamePaused true)
  (return))