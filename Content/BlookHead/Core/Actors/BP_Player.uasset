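; BP_Player is the physics-driven player cube that constantly pushes forward through a level toward an end point.
; Tick applies forward acceleration while the level is in play, and Enhanced Input adds left/right force.
; Hitting a BP_Obstacle (after a delay) or falling below KillZ calls PlayerDied, which stops play and prints Game Over.
; Overlapping BP_EndPoint stops play and notifies BP_GameMode that the level is complete.
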(event OnComponentBeginOverlap(Cube)
  (params (OverlappedComponent :type Primitive%20Component%20Object%20Reference) (OtherActor :type Actor%20Object%20Reference) (OtherComp :type Primitive%20Component%20Object%20Reference) (OtherBodyIndex :type Integer) (bFromSweep :type Boolean) (SweepResult :type Hit%20Result%20Structure%20%28by%20ref%29))
  (Utilities|Casting|CastToBP_EndPoint OtherActor)
  (Development|PrintString "You  Win")
  (Variables|Default|SetbLevelInPlayer false)
  (Default|LevelComplete (Variables|Default|GetGameMode)))

(event OnComponentHit(Cube)
  (params (HitComponent :type Primitive%20Component%20Object%20Reference) (OtherActor :type Actor%20Object%20Reference) (OtherComp :type Primitive%20Component%20Object%20Reference) (NormalImpulse :type Vector :default "0, 0, 0") (Hit :type Hit%20Result%20Structure%20%28by%20ref%29))
  (Utilities|Casting|CastToBP_Obstacle OtherActor)
  (Development|PrintString "You hit me")
  (Utilities|FlowControl|Delay (Variables|Default|GetPostHitDelay))
  (CallFunction|PlayerDied))

(event Input|EnhancedActionEvents|EnhancedInputActionIA_MoveRigthLeft
  (params (ActionValue :type Float%20%28double-precision%29) (ElapsedSeconds :type Float%20%28double-precision%29) (TriggeredSeconds :type Float%20%28double-precision%29) (InputAction :type Input%20Action%20Object%20Reference :default "/Game/BlookHead/Input/Actions/IA_MoveRigthLeft.IA_MoveRigthLeft"))
  (if (Variables|Default|GetbLevelInPlayer)
    (Physics|AddForce (Variables|Default|GetCube) (* (* ActionValue (Transformation|GetActorRightVector)) (Variables|Movement|GetRightSpeed)) "None" true)))

(event EventBeginPlay
  (Utilities|FlowControl|Sequence
    (:then_0
      (bind _asplayer_controller (Utilities|Casting|CastToPlayerController (Pawn|GetController))
        (:then
          (Variables|Default|SetPlayerController _asplayer_controller)
          (Input|AddMappingContext (PlayerController|LocalPlayerSubsystems|GetEnhancedInputLocalPlayerSubsystem (Variables|Default|GetPlayerController)) "/Game/BlookHead/Input/IMC_Mappings.IMC_Mappings" 0 "(bIgnoreAllPressedKeysUntilRelease=True,bForceImmediately=False,bNotifyUserSettings=False)"))
        (:CastFailed
          (Development|PrintString "Controller Cast Failed"))))
    (:then_1
      (bind _asbp_game_mode (Utilities|Casting|CastToBP_GameMode (Game|GetGameMode)))
      (Variables|Default|SetGameMode _asbp_game_mode))))

(event EventTick
  (params (DeltaSeconds :type Float%20%28single-precision%29))
  (Utilities|FlowControl|Sequence
    (:then_0
      (if (Variables|Default|GetbLevelInPlayer)
        (Physics|AddForce (Variables|Default|GetCube) (* (Transformation|GetActorForwardVector) (Variables|Movement|GetForwardSpeed)) "None" true)))
    (:then_1
      (if (< (.z (Transformation|GetActorLocation)) (Variables|Default|GetKillZ))
        (CallFunction|PlayerDied)))))

(fn ConstructionScript)

(fn PlayerDied
  (if (Variables|Default|GetbLevelInPlayer)
    (Variables|Default|SetbLevelInPlayer false)
    (Development|PrintString "Game Over")
    (return)))